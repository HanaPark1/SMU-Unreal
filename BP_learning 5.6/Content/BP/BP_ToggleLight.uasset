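; BP_ToggleLight is a point light actor that switches on while something overlaps its Box trigger and off when the overlap ends.
; The construction script applies the LightVisibility, LightIntensity and LightColor variables to the point light.
; The Box begin and end overlap events set the light's visibility directly, with no check on which actor overlaps, and BeginPlay and Tick are unused.
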(event `self.Box.OnComponentBeginOverlap`
  (params (OverlappedComponent :type "PrimitiveComponent Object Reference") (OtherActor :type "Actor Object Reference") (OtherComp :type "PrimitiveComponent Object Reference") (OtherBodyIndex :type Integer) (bFromSweep :type Boolean) (SweepResult :type "HitResult Structure (by ref)"))
  (`SceneComponent.SetVisibility` (`self.PointLightComponent`) true false))

(event `self.Box.OnComponentEndOverlap`
  (params (OverlappedComponent :type "PrimitiveComponent Object Reference") (OtherActor :type "Actor Object Reference") (OtherComp :type "PrimitiveComponent Object Reference") (OtherBodyIndex :type Integer))
  (`SceneComponent.SetVisibility` (`self.PointLightComponent`) false false))

(fn `UserConstructionScript`
  (bind _pointlightcomponent (`self.PointLightComponent`))
  (`SceneComponent.SetVisibility` _pointlightcomponent (`self.Light Visibility`) false)
  (`LightComponent.SetIntensity` _pointlightcomponent (`self.Light Intensity`))
  (`LightComponent.SetLightColor` _pointlightcomponent (`self.Light Color`) true))